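; BP_PetPawn is the pet pawn, exposing movement commands to walk to an actor, walk to a location, stop walking and set a crouch state.
; Both walk events snap rotation toward the destination, run AIMoveTo, then fire OnActionSucceeded or OnActionFailed to report the result.
; Stopping halts movement through the controller, while the crouch event only stores the IsCrouch flag.
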(event `self.ReceiveBeginPlay`)

(event `self.ReceiveTick`
  (params (DeltaSeconds :type "Float (single-precision)")))

(event `self.WalkToTarget`
  (params (Target :type "Actor Object Reference"))
  (`self.K2_SetActorRotation` (`KismetMathLibrary.FindLookAtRotation` (`self.K2_GetActorLocation`) (`self.K2_GetActorLocation` Target)))
  (`|AIMoveTo` self (0.0 0.0 0.0) Target 100.0
    (:`OnSuccess`
      (`self.OnActionSucceeded`))
    (:`OnFail`
      (`self.OnActionFailed`))))

(event `self.StopWalk`
  (`Controller.StopMovement` (`self.GetController`)))

(event `self.WalkInLocation`
  (params (InLocation :type "Vector Structure"))
  (`self.K2_SetActorRotation` (`KismetMathLibrary.FindLookAtRotation` (`self.K2_GetActorLocation`) InLocation))
  (`|AIMoveTo` self InLocation null
    (:`OnSuccess`
      (`self.OnActionSucceeded`))
    (:`OnFail`
      (`self.OnActionFailed`))))

(event `self.SetCrouchState`
  (params (bInCrouch :type Boolean))
  (set `self.bIsCrouch` bInCrouch))

(fn `UserConstructionScript`)